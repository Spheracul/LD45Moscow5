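; BP_Door is a level door that slides its mesh down when the player approaches and back up afterwards.
; Front and back trigger boxes open it for the player character, driving a reversible timeline.
; On exit from either box, it closes unless the other box's CookieJar-filtered overlaps contain the exiting actor.
; Any back-box overlap also sends DoorToGenRoomMessage to the parent actor.
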(event `OpenOrClose`
  (params (`Open?` :type Boolean))
  (if `Open?`
    (bind (_direction _tltime) (`Timeline|DoorTL` :!label _label)
      (:`Update`
        (`SceneComponent.K2_SetRelativeLocation` (`self.StaticMesh`) (`KismetMathLibrary.MakeVector` 0.0 0.0 (* _tltime -248.0)) false false)))
    (else
      (goto _label :!via `Reverse`))))

(event `self.BoxFront.OnComponentBeginOverlap`
  (params (OverlappedComponent :type "PrimitiveComponent Object Reference") (OtherActor :type "Actor Object Reference") (OtherComp :type "PrimitiveComponent Object Reference") (OtherBodyIndex :type Integer) (bFromSweep :type Boolean) (SweepResult :type "HitResult Structure (by ref)"))
  (`self.CheckIfCanOpen` OtherActor))

(event `self.BoxBack.OnComponentBeginOverlap`
  (params (OverlappedComponent :type "PrimitiveComponent Object Reference") (OtherActor :type "Actor Object Reference") (OtherComp :type "PrimitiveComponent Object Reference") (OtherBodyIndex :type Integer) (bFromSweep :type Boolean) (SweepResult :type "HitResult Structure (by ref)"))
  (`self.CheckIfCanOpen` OtherActor)
  (message `/Game/LevelActors/Cookie_Interface.DoorToGenRoom` (`self.GetParentActor`) null))

(event `self.BoxFront.OnComponentEndOverlap`
  (params (OverlappedComponent :type "PrimitiveComponent Object Reference") (OtherActor :type "Actor Object Reference") (OtherComp :type "PrimitiveComponent Object Reference") (OtherBodyIndex :type Integer))
  (`self.CheckIfCanClose` (`self.BoxBack`) OtherActor))

(event `self.BoxBack.OnComponentEndOverlap`
  (params (OverlappedComponent :type "PrimitiveComponent Object Reference") (OtherActor :type "Actor Object Reference") (OtherComp :type "PrimitiveComponent Object Reference") (OtherBodyIndex :type Integer))
  (`self.CheckIfCanClose` (`self.BoxFront`) OtherActor))

(fn `CheckIfCanClose`
  (params (OtherCollider :type "PrimitiveComponent Object Reference") (TriggeringActor :type "Actor Object Reference (by ref)"))
  (if (not (`KismetArrayLibrary.Array_Contains` (`PrimitiveComponent.GetOverlappingActors` OtherCollider "/Game/LevelActors/Characters/CookieJar.CookieJar_C") TriggeringActor))
    (`self.OpenOrClose` false)))

(fn `CheckIfCanOpen`
  (params (Actor :type "Object Object Reference"))
  (if (== Actor (`GameplayStatics.GetPlayerCharacter` 0))
    (`self.OpenOrClose` true)))

(fn `UserConstructionScript`)